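; Player build component for BP_FirstPersonCharacter that previews, rotates and places tiles from a data table, with preview logic only for Piles so far.
; Gameplay tags track build/adjust modes and validity, driving the preview material each tick.
; Camera traces position a Pile, then adjust mode sets its height using closest-point math between view ray and vertical axis.
; Placed Piles spawn capsule snap points that snap, height-match or invalidate nearby previews, with a secondary ghost mesh.
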(event Custom|SecondaryPreviewMeshLoop
  ;[1 1 1] Add/Reset the Secondary Preview Mesh
  (Utilities|FlowControl|Sequence
    (:then_0
      (Utilities|FlowControl|DoOnce false
        (:Completed
          (Components|StaticMesh|SetStaticMesh (Variables|SecondaryPreviewMesh|GetSecondaryPreviewMesh) (.mesh (Helpers|GetSelectedTile)))
          (Rendering|Material|SetMaterial (Variables|SecondaryPreviewMesh|GetSecondaryPreviewMesh) 0 "/Game/BuildingSystem/Materials/BuildPreview/MI_BuildPreview_Temporary.MI_BuildPreview_Temporary"))))
    (:then_1
      (Utilities|IsValid (Variables|/Script/Engine.StaticMeshComponent|GetStaticMesh (Variables|SecondaryPreviewMesh|GetSecondaryPreviewMesh))
        (:Is%20Valid
          (Transformation|SetWorldTransform (Variables|SecondaryPreviewMesh|GetSecondaryPreviewMesh) (Math|Transform|MakeTransform (Variables|SecondaryPreviewMesh|GetSecondaryPreviewMeshLocation) (Variables|SecondaryPreviewMesh|GetSecondaryPreviewMeshRotation) (Variables|SecondaryPreviewMesh|GetSecondaryPreviewMeshScale)) false false))))))

(event Custom|ResetSecondaryPreviewMesh
  ;[1 1 1] Add/Reset the Secondary Preview Mesh
  (Components|StaticMesh|SetStaticMesh (Variables|SecondaryPreviewMesh|GetSecondaryPreviewMesh) 0)
  (Utilities|FlowControl|DoOnce false) ; enters at Reset
)

(event Custom|PreviewMeshLoop
  ;[1 1 1] Add/Reset Preview Mesh
  (Utilities|FlowControl|DoOnce false
    (:Completed
      (Components|StaticMesh|SetStaticMesh (Variables|PreviewMesh|GetPreviewMesh) (.mesh (Helpers|GetSelectedTile)))
      (Variables|Runtime|SetPreviewTransformValidation "(TagName=\"PreviewState.Valid\")"))))

(event Custom|ResetPreviewMesh
  ;[1 1 1] Add/Reset Preview Mesh
  (Components|StaticMesh|SetStaticMesh (Variables|PreviewMesh|GetPreviewMesh) 0)
  (Utilities|FlowControl|DoOnce false) ; enters at Reset
)

(event Input|EnhancedActionEvents|EnhancedInputActionIA_ScrollWithShift
  (params (ActionValue :type Float%20%28double-precision%29) (ElapsedSeconds :type Float%20%28double-precision%29) (TriggeredSeconds :type Float%20%28double-precision%29) (InputAction :type Input%20Action%20Object%20Reference :default "/Game/FirstPerson/Input/Actions/IA_ScrollWithShift.IA_ScrollWithShift"))
  (:Triggered
    (Variables|Runtime|SetTraceForwardLength (Math|Float|Clamp(Float) (- (Variables|Runtime|GetTraceForwardLength) (* ActionValue (Variables|InternalSettings|GetTraceForwardSensitivity))) 2.5e+02 7e+02))))

(event Input|EnhancedActionEvents|EnhancedInputActionIA_PlaceBuild
  (params (ActionValue :type Boolean) (ElapsedSeconds :type Float%20%28double-precision%29) (TriggeredSeconds :type Float%20%28double-precision%29) (InputAction :type Input%20Action%20Object%20Reference :default "/Game/FirstPerson/Input/Actions/IA_PlaceBuild.IA_PlaceBuild"))
  (bind _selectedtile (Helpers|GetSelectedTile))
  ;[1 1 1] Tile Placement
  (:Completed
    (if (and (Helpers|InBuildMode) (Helpers|TransformValid))
      (switch Utilities|FlowControl|Switch|SwitchonETileName (.name (Helpers|GetSelectedTile))
        (:NewEnumerator1
          (if (Helpers|InAdjustMode)
            (bind _returnvalue (Game|SpawnActorfromClass (.blueprint (Helpers|GetSelectedTile)) (Math|Transform|MakeTransform (Variables|PreviewMesh|GetPreviewMeshLocation) (Variables|PreviewMesh|GetPreviewMeshRotation)) "AlwaysSpawn" "MultiplyWithRoot" 0 0 :!label _label))
            (Utilities|FlowControl|Sequence
              (:then_0
                (Transformation|SetWorldScale3D (Variables|/Game/BuildingSystem/Blueprints/Tiles/BP_BuildMaster.BP_BuildMaster_C|GetMesh _returnvalue) (Variables|PreviewMesh|GetPreviewMeshScale))
                (SnapPointManagement|ProcessNewTile _returnvalue (.name _selectedtile))
                (bind _returnvalue_2 (Rendering|Material|CreateDynamicMaterialInstance (Variables|/Game/BuildingSystem/Blueprints/Tiles/BP_BuildMaster.BP_BuildMaster_C|GetMesh _returnvalue) 0 (.material _selectedtile) "None" :!class /Script/Engine.PrimitiveComponent))
                (Rendering|Material|SetScalarParameterValue _returnvalue_2 "SizeV" (.Z (Math|Vector|BreakVector (Variables|PreviewMesh|GetPreviewMeshScale))) :!class /Script/Engine.MaterialInstanceDynamic)
                (Variables|Runtime|SetPreviewTransformValidation "(TagName=\"PreviewState.Invalid\")"))
              (:then_1
                (Variables|Runtime|SetPlayerMode "(TagName=\"PlayerState.BuildMode\")")
                (Utilities|FlowControl|Sequence
                  (:then_0
                    (Variables|PreviewMesh|SetPreviewMeshLocation "0, 0, 0"))
                  (:then_1
                    (Variables|PreviewMesh|SetPreviewMeshRotation "0, 0, 0"))
                  (:then_2
                    (Variables|PreviewMesh|SetPreviewMeshScale "1.000000,1.000000,1.000000")))))
            (else
              (Variables|Runtime|SetPlayerMode "(TagName=\"PlayerState.BuildMode.AdjustMode\")"))))
        (:NewEnumerator2
          (goto _label))))))

(event Input|EnhancedActionEvents|EnhancedInputActionIA_RotateBuildPreview
  (params (ActionValue :type Float%20%28double-precision%29) (ElapsedSeconds :type Float%20%28double-precision%29) (TriggeredSeconds :type Float%20%28double-precision%29) (InputAction :type Input%20Action%20Object%20Reference :default "/Game/FirstPerson/Input/Actions/IA_RotateBuildPreview.IA_RotateBuildPreview"))
  ;[1 1 1] Tile Preview Rotation Logic
  (if (Helpers|InBuildMode)
    (if (not (Helpers|InAdjustMode))
      (Variables|PreviewMesh|SetPreviewMeshRotation (Math|Rotator|MakeRotator (.roll (Variables|PreviewMesh|GetPreviewMeshRotation)) (.pitch (Variables|PreviewMesh|GetPreviewMeshRotation)) (+ (.yaw (Variables|PreviewMesh|GetPreviewMeshRotation)) (* ActionValue (Variables|InternalSettings|GetPreviewRotationSensitivity))))))))

(event Input|EnhancedActionEvents|EnhancedInputActionIA_ToggleBuildMode
  (params (ActionValue :type Boolean) (ElapsedSeconds :type Float%20%28double-precision%29) (TriggeredSeconds :type Float%20%28double-precision%29) (InputAction :type Input%20Action%20Object%20Reference :default "/Game/FirstPerson/Input/Actions/IA_ToggleBuildMode.IA_ToggleBuildMode"))
  ;[1 1 1] Toggle Build Mode
  (:Started
    (Toggle|ToggleBuildMode)))

(event Input|EnhancedActionEvents|EnhancedInputActionIA_NextTile
  (params (ActionValue :type Boolean) (ElapsedSeconds :type Float%20%28double-precision%29) (TriggeredSeconds :type Float%20%28double-precision%29) (InputAction :type Input%20Action%20Object%20Reference :default "/Game/FirstPerson/Input/Actions/IA_NextTile.IA_NextTile"))
  (bind _selectedtile (Helpers|GetSelectedTile))
  ;[1 1 1] Iteration through the tiles
  (:Started
    (if (not (Helpers|InAdjustMode))
      (bind _outrownames (DataTable|GetDataTableRowNames "/Game/BuildingSystem/FAvailableTiles.FAvailableTiles"))
      (if (== (Variables|Runtime|GetTileSelection) (- (Utilities|Array|Length _outrownames) 1))
        (Variables|Runtime|SetTileSelection 0)
        (else
          (Math|Integer|IncrementInt (Variables|Runtime|GetTileSelection)
            (:%20%20
              _))))
      (Components|StaticMesh|SetStaticMesh (Variables|PreviewMesh|GetPreviewMesh) (.mesh _selectedtile))
      (Components|StaticMesh|SetStaticMesh (Variables|SecondaryPreviewMesh|GetSecondaryPreviewMesh) (.mesh _selectedtile)))))

(event Input|EnhancedActionEvents|EnhancedInputActionIA_PrevTile
  (params (ActionValue :type Boolean) (ElapsedSeconds :type Float%20%28double-precision%29) (TriggeredSeconds :type Float%20%28double-precision%29) (InputAction :type Input%20Action%20Object%20Reference :default "/Game/FirstPerson/Input/Actions/IA_PrevTile.IA_PrevTile"))
  (bind _selectedtile (Helpers|GetSelectedTile))
  ;[1 1 1] Iteration through the tiles
  (:Started
    (if (not (Helpers|InAdjustMode))
      (if (== (Variables|Runtime|GetTileSelection) 0)
        (bind _outrownames (DataTable|GetDataTableRowNames "/Game/BuildingSystem/FAvailableTiles.FAvailableTiles"))
        (Variables|Runtime|SetTileSelection (- (Utilities|Array|Length _outrownames) 1))
        (else
          (Math|Integer|DecrementInt (Variables|Runtime|GetTileSelection)
            (:%20%20
              _))))
      (Components|StaticMesh|SetStaticMesh (Variables|PreviewMesh|GetPreviewMesh) (.mesh _selectedtile))
      (Components|StaticMesh|SetStaticMesh (Variables|SecondaryPreviewMesh|GetSecondaryPreviewMesh) (.mesh _selectedtile)))))

(event EventBeginPlay
  ;[1 1 1] BeginPlay and Tick
  (bind _asbp_first_person_character (Utilities|Casting|CastToBP_FirstPersonCharacter (Components|GetOwner)))
  (bind _output_get (Variables|External|SetCharacterBP _asbp_first_person_character))
  (Variables|External|SetBP_Camera (Variables|/Script/BuildingSystem.BuildingSystemCharacter|GetFirstPersonCameraComponent _output_get))
  (bind _returnvalue (Game|AddComponentbyClass (Variables|External|GetCharacterBP) "/Script/Engine.StaticMeshComponent" false))
  (bind _output_get_2 (Variables|PreviewMesh|SetPreviewMesh _returnvalue))
  (bind _returnvalue_2 (Rendering|Material|CreateDynamicMaterialInstance _output_get_2 0 "/Game/BuildingSystem/Materials/BuildPreview/MI_BuildPreview.MI_BuildPreview" "" :!class /Script/Engine.PrimitiveComponent))
  (bind _output_get_3 (Variables|PreviewMesh|SetPreviewMeshMaterial _returnvalue_2))
  (Rendering|Material|SetMaterial (Variables|PreviewMesh|GetPreviewMesh) 0 _output_get_3)
  (Collision|SetCollisionEnabled (Variables|PreviewMesh|GetPreviewMesh) "NoCollision")
  (bind _returnvalue_3 (Game|AddComponentbyClass (Variables|External|GetCharacterBP) "/Script/Engine.StaticMeshComponent" false))
  (bind _output_get_4 (Variables|SecondaryPreviewMesh|SetSecondaryPreviewMesh _returnvalue_3))
  (Collision|SetCollisionEnabled _output_get_4 "NoCollision"))

(event EventTick
  (params (DeltaSeconds :type Float%20%28single-precision%29))
  ;[1 1 1] BeginPlay and Tick
  (if (Helpers|InBuildMode)
    (Loops|TilePreviewLoop)))

(fn FindClosestPointsSegmenttoLine
  (params (SegmentStart :type Vector) (SegmentEnd :type Vector) (LineStart :type Vector) (LineDirection :type Vector))
  (Utilities|FlowControl|Sequence
    (:then_0
      (LocalVariables|SetA0 SegmentStart)
      (LocalVariables|SetB0 LineStart)
      (LocalVariables|SetVa (- SegmentEnd SegmentStart))
      (LocalVariables|SetVb LineDirection)
      (LocalVariables|Setr (- (LocalVariables|GetA0) (LocalVariables|GetB0))))
    (:then_1
      (LocalVariables|Seta (Math|Vector|DotProduct (LocalVariables|GetVa) (LocalVariables|GetVa)))
      (LocalVariables|Setb (Math|Vector|DotProduct (LocalVariables|GetVa) (LocalVariables|GetVb)))
      (LocalVariables|Setc (Math|Vector|DotProduct (LocalVariables|GetVb) (LocalVariables|GetVb)))
      (LocalVariables|Setd (Math|Vector|DotProduct (LocalVariables|GetVa) (LocalVariables|Getr)))
      (LocalVariables|Sete (Math|Vector|DotProduct (LocalVariables|GetVb) (LocalVariables|Getr)))
      (LocalVariables|Setdelta (- (* (LocalVariables|Geta) (LocalVariables|Getc)) (* (LocalVariables|Getb) (LocalVariables|Getb)))))
    (:then_2
      (LocalVariables|Setp (/ (- (* (LocalVariables|Getb) (LocalVariables|Gete)) (* (LocalVariables|Getc) (LocalVariables|Getd))) (LocalVariables|Getdelta)))
      (LocalVariables|Setq (/ (- (* (LocalVariables|Geta) (LocalVariables|Gete)) (* (LocalVariables|Getb) (LocalVariables|Getd))) (LocalVariables|Getdelta)))
      (LocalVariables|SetSegmentPoint (+ (LocalVariables|GetA0) (* (LocalVariables|GetVa) (LocalVariables|Getp))))
      (LocalVariables|SetLinePoint (+ (LocalVariables|GetB0) (* (LocalVariables|GetVb) (LocalVariables|Getq))))
      (return (LocalVariables|GetSegmentPoint) (LocalVariables|GetLinePoint)))))

(fn GetScalebyTopPoint
  (params (TargetPoint :type Vector))
  (bind _previewmesh (Variables|PreviewMesh|GetPreviewMesh))
  (bind (_min _max) (Components|StaticMesh|GetLocalBounds _previewmesh))
  (if (Utilities|IsValid (Variables|PreviewMesh|GetPreviewMesh))
    (Utilities|FlowControl|Sequence
      (:then_0
        (LocalVariables|SetOriginalHeight (- (.z _max) (.z _min))))
      (:then_1
        (LocalVariables|SetTargetHeight (Math|Float|Clamp(Float) (- (.z TargetPoint) (.z (Transformation|GetWorldLocation (Variables|PreviewMesh|GetPreviewMesh)))) 0.1 (* 2.0 (Variables|Constants|GetCellSideLength)))))
      (:then_2
        (return (Math|Vector|MakeVector 1.0 1.0 (/ (LocalVariables|GetTargetHeight) (LocalVariables|GetOriginalHeight))))))))

(fn GetSelectedTile
  (bind _outrownames (DataTable|GetDataTableRowNames "/Game/BuildingSystem/FAvailableTiles.FAvailableTiles"))
  (bind _returnvalue (Utilities|GetDataTableRow "/Game/BuildingSystem/FAvailableTiles.FAvailableTiles" (Utilities|Array|Get(acopy) _outrownames (Variables|Runtime|GetTileSelection)))
    (:then
      (return (Utilities|Struct|MakeFTile (.name _returnvalue) (.mesh _returnvalue) (.material _returnvalue) (.blueprint _returnvalue))))))

(fn InBuildMode
  (return (GameplayTags|MatchesTag (Variables|Runtime|GetPlayerMode) "(TagName=\"PlayerState.BuildMode\")")))

(fn InAdjustMode
  (return (GameplayTags|MatchesTag (Variables|Runtime|GetPlayerMode) "(TagName=\"PlayerState.BuildMode.AdjustMode\")" true)))

(fn TransformValid
  (return (GameplayTags|MatchesTag (Variables|Runtime|GetPreviewTransformValidation) "(TagName=\"PreviewState.Valid\")" true)))

(fn TransformInvalid
  (return (GameplayTags|MatchesTag (Variables|Runtime|GetPreviewTransformValidation) "(TagName=\"PreviewState.Invalid\")" true)))

(fn TilePreviewLoop
  (CallFunction|PreviewMeshLoop)
  (Utilities|IsValid (Variables|/Script/Engine.StaticMeshComponent|GetStaticMesh (Variables|PreviewMesh|GetPreviewMesh))
    (:Is%20Valid
      (Transformation|SetWorldTransform (Variables|PreviewMesh|GetPreviewMesh) (Math|Transform|MakeTransform (Variables|PreviewMesh|GetPreviewMeshLocation) (Variables|PreviewMesh|GetPreviewMeshRotation) (Variables|PreviewMesh|GetPreviewMeshScale)) false false)
      (|SwitchGameplayTag (Variables|Runtime|GetPreviewTransformValidation)
        (:Default
          (Rendering|Material|SetScalarParameterValue (Variables|PreviewMesh|GetPreviewMeshMaterial) "Value" 0.0 :!class /Script/Engine.MaterialInstanceDynamic :!label _label))
        (:PreviewState.Invalid
          (goto _label))
        (:PreviewState.Partial
          (Rendering|Material|SetScalarParameterValue (Variables|PreviewMesh|GetPreviewMeshMaterial) "Value" (Variables|Runtime|GetPartialPreviewValue) :!class /Script/Engine.MaterialInstanceDynamic))
        (:PreviewState.Valid
          (Rendering|Material|SetScalarParameterValue (Variables|PreviewMesh|GetPreviewMeshMaterial) "Value" 1.0 :!class /Script/Engine.MaterialInstanceDynamic)))
      (switch Utilities|FlowControl|Switch|SwitchonETileName (.name (Helpers|GetSelectedTile))
        (:NewEnumerator1
          (if (Helpers|InAdjustMode)
            (|PileAdjustMode)
            (else
              (|PilePreviewMode)))
          (SnapPointManagement|CheckSnaps))))))

(fn ToggleBuildMode
  (if (Helpers|InBuildMode)
    (Variables|Runtime|SetPlayerMode "(TagName=\"\")")
    (CallFunction|ResetPreviewMesh)
    (else
      (Variables|Runtime|SetPlayerMode "(TagName=\"PlayerState.BuildMode\")")
      (CallFunction|PreviewMeshLoop))))

(fn ProcessNewTile
  (params (TileReference :type BP%20Build%20Master%20Object%20Reference) (TileType :type ETileName%20Enum :default "NewEnumerator1"))
  (bind _cellsidelength (Variables|Constants|GetCellSideLength))
  (bind _returnvalue (Transformation|GetActorLocation TileReference))
  (bind _boxextent (Collision|GetActorBounds TileReference false false))
  (bind (_x _y _z) (Math|Vector|BreakVector _returnvalue))
  (bind _returnvalue_2 (* (.z _boxextent) 2.0))
  (bind _returnvalue_3 (/ _returnvalue_2 2.0))
  (switch Utilities|FlowControl|Switch|SwitchonETileName TileType
    (:NewEnumerator1
      (bind _returnvalue_4 (Game|SpawnActorfromClass "/Game/BuildingSystem/Blueprints/SnapPoints/BP_CapsuleSnapPoint.BP_CapsuleSnapPoint_C" (Math|Transform|MakeTransform (Math|Vector|MakeVector _x _y (+ _z _returnvalue_3))) "Undefined" "MultiplyWithRoot" 0 0))
      (Class|BPIBuildInterface|AddSnapPointTags(Message) _returnvalue_4 "(GameplayTags=((TagName=\"Snap.Support\")))")
      (Components|Capsule|SetCapsuleSize (Variables|/Game/BuildingSystem/Blueprints/SnapPoints/BP_CapsuleSnapPoint.BP_CapsuleSnapPoint_C|GetCapsule _returnvalue_4) _cellsidelength (+ _returnvalue_3 _cellsidelength) true))))

(fn CheckSnaps
  (switch Utilities|FlowControl|Switch|SwitchonETileName (.name (Helpers|GetSelectedTile))
    (:NewEnumerator1
      (bind _outactors (Collision|SphereOverlapActors (Variables|PreviewMesh|GetPreviewMeshLocation) (Variables|InternalSettings|GetCheckRadius_Pile) (Utilities|Array|MakeArray "ObjectTypeQuery8") "/Game/BuildingSystem/Blueprints/SnapPoints/BP_CapsuleSnapPoint.BP_CapsuleSnapPoint_C"))
      (if (.NotEmpty (SnapPointManagement|FilterSnapPoints _outactors "(GameplayTags=((TagName=\"Snap.Support\")))"))
        (bind _capsule (Class|BPISnapCapsule|GetCapsule(Message) (.ReturnValue (Actor|FindNearestActor (Variables|PreviewMesh|GetPreviewMeshLocation) (.FilteredSnapPoints (SnapPointManagement|FilterSnapPoints _outactors "(GameplayTags=((TagName=\"Snap.Support\")))"))))))
        (bind _output_get (LocalVariables|SetTargetCapsule _capsule))
        (LocalVariables|SetBottom (+ (Transformation|GetWorldLocation _output_get) (* (- (Components|Capsule|GetScaledCapsuleHalfHeight _output_get) (Components|Capsule|GetScaledCapsuleRadius _output_get)) "0.000000,0.000000,-1.000000")))
        (bind _output_get_2 (LocalVariables|SetTop (+ (Transformation|GetWorldLocation _output_get) (* (- (Components|Capsule|GetScaledCapsuleHalfHeight _output_get) (Components|Capsule|GetScaledCapsuleRadius _output_get)) "0.000000,0.000000,1.000000"))))
        (bind _output_get_3 (Variables|PreviewMesh|SetPreviewMeshScale (Helpers|GetScalebyTopPoint _output_get_2)))
        (Variables|SecondaryPreviewMesh|SetSecondaryPreviewMeshScale _output_get_3)
        (bind _output_get_4 (LocalVariables|SetProjection (Math|Vector|FindClosestPointonSegment (Variables|PreviewMesh|GetPreviewMeshLocation) (LocalVariables|GetBottom) (LocalVariables|GetTop))))
        (bind _output_get_5 (LocalVariables|SetSnapPointBaseDistance (Math|Float|MapRangeClamped (Math|Vector|Distance(Vector) _output_get_4 (Variables|PreviewMesh|GetPreviewMeshLocation)) 0.0 (Variables|Constants|GetCellSideLength) 0.0 1.0)))
        (if (>= _output_get_5 0.94)
          (CallFunction|ResetSecondaryPreviewMesh)
          (Variables|PreviewMesh|SetPreviewMeshLocation (+ (LocalVariables|GetProjection) (* (Math|Vector|Normalize (- (Variables|PreviewMesh|GetPreviewMeshLocation) (LocalVariables|GetProjection))) (Components|Capsule|GetScaledCapsuleRadius (LocalVariables|GetTargetCapsule)))))
          (elif (>= (LocalVariables|GetSnapPointBaseDistance) 0.65)
            (CallFunction|SecondaryPreviewMeshLoop)
            (Variables|Runtime|SetPreviewTransformValidation "(TagName=\"PreviewState.Partial\")")
            (Variables|Runtime|SetPartialPreviewValue (Math|Float|MapRangeClamped (LocalVariables|GetSnapPointBaseDistance) 0.65 0.94 0.0 1.0))
            (Variables|SecondaryPreviewMesh|SetSecondaryPreviewMeshLocation (+ (LocalVariables|GetProjection) (* (Math|Vector|Normalize (- (Variables|PreviewMesh|GetPreviewMeshLocation) (LocalVariables|GetProjection))) (Components|Capsule|GetScaledCapsuleRadius (LocalVariables|GetTargetCapsule)))))
            (else
              (CallFunction|ResetSecondaryPreviewMesh)
              (Variables|Runtime|SetPreviewTransformValidation "(TagName=\"PreviewState.Invalid\")"))))
        (elif (not (Helpers|InAdjustMode))
          (bind _output_get_6 (Variables|PreviewMesh|SetPreviewMeshScale "1.000000,1.000000,1.000000"))
          (Variables|SecondaryPreviewMesh|SetSecondaryPreviewMeshScale _output_get_6))))))

(fn FilterSnapPoints
  (params (Actors :type Array%20of%20Actor%20Object%20References) (Tags :type Gameplay%20Tag%20Container%20Structure))
  (bind _filteredsnaps (LocalVariables|GetFilteredSnaps))
  (for _array_element Actors
    (if (Utilities|DoesObjectImplementInterface _array_element "/Game/BuildingSystem/Blueprints/BPI_BuildInterface.BPI_BuildInterface_C")
      (bind _tags (Class|BPIBuildInterface|GetSnapPointTags(Message) _array_element))
      (if (GameplayTags|HasAnyTags _tags Tags true)
        (Utilities|Array|AddUnique (LocalVariables|GetFilteredSnaps) _array_element))))
  (return _filteredsnaps (> (Utilities|Array|Length _filteredsnaps) 0)))