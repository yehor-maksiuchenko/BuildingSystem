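; Building-system manager that creates snap points for placed tiles and computes snapped placement for new ones, currently handling only Pile tiles.
; ProcessNewTile spawns a Snap.Support capsule spanning the pile's height.
; CheckSnaps sphere-overlaps for tagged capsules, then snaps one cell length from the nearest, keeping approach direction and clamping Z to its bounds.
; The older eight-neighbour cube-snap pile processing remains but is disconnected.
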(event EventBeginPlay)

(event Collision|EventActorBeginOverlap
  (params (OtherActor :type Actor%20Object%20Reference)))

(event EventTick
  (params (DeltaSeconds :type Float%20%28single-precision%29)))

(fn ConstructionScript)

(fn CheckSnaps
  (params (InLocation :type Vector) (InRotation :type Rotator) (InScale :type Vector) (Tile :type ETileName%20Enum :default "NewEnumerator1"))
  (switch Utilities|FlowControl|Switch|SwitchonETileName Tile
    (:NewEnumerator1
      (bind (_outactors _returnvalue) (Collision|SphereOverlapActors InLocation (Variables|Constants|GetCheckRadius_Pile) (Utilities|Array|MakeArray "ObjectTypeQuery8") "/Game/BuildingSystem/Blueprints/SnapPoints/BP_CapsuleSnapPoint.BP_CapsuleSnapPoint_C"))
      (if (and (.NotEmpty (CallFunction|FilterSnapPoints _outactors "(GameplayTags=((TagName=\"Snap.Support\")))")) _returnvalue)
        (return true (Math|Transform|MakeTransform (Math|Vector|MakeVector (.x (+ (* (Math|Vector|GetUnitDirection(Vector) (Transformation|GetActorLocation (.ReturnValue (Actor|FindNearestActor InLocation (.FilteredSnapPoints (CallFunction|FilterSnapPoints _outactors "(GameplayTags=((TagName=\"Snap.Support\")))"))))) InLocation) (Variables|Constants|GetCellSideLength)) (Transformation|GetActorLocation (.ReturnValue (Actor|FindNearestActor InLocation (.FilteredSnapPoints (CallFunction|FilterSnapPoints _outactors "(GameplayTags=((TagName=\"Snap.Support\")))"))))))) (.y (+ (* (Math|Vector|GetUnitDirection(Vector) (Transformation|GetActorLocation (.ReturnValue (Actor|FindNearestActor InLocation (.FilteredSnapPoints (CallFunction|FilterSnapPoints _outactors "(GameplayTags=((TagName=\"Snap.Support\")))"))))) InLocation) (Variables|Constants|GetCellSideLength)) (Transformation|GetActorLocation (.ReturnValue (Actor|FindNearestActor InLocation (.FilteredSnapPoints (CallFunction|FilterSnapPoints _outactors "(GameplayTags=((TagName=\"Snap.Support\")))"))))))) (Math|Float|Clamp(Float) (.Z (Math|Vector|BreakVector InLocation)) (- (.z (.Origin (Collision|GetActorBounds (.ReturnValue (Actor|FindNearestActor InLocation (.FilteredSnapPoints (CallFunction|FilterSnapPoints _outactors "(GameplayTags=((TagName=\"Snap.Support\")))")))) false false))) (.z (.BoxExtent (Collision|GetActorBounds (.ReturnValue (Actor|FindNearestActor InLocation (.FilteredSnapPoints (CallFunction|FilterSnapPoints _outactors "(GameplayTags=((TagName=\"Snap.Support\")))")))) false false)))) (+ (.z (.Origin (Collision|GetActorBounds (.ReturnValue (Actor|FindNearestActor InLocation (.FilteredSnapPoints (CallFunction|FilterSnapPoints _outactors "(GameplayTags=((TagName=\"Snap.Support\")))")))) false false))) (.z (.BoxExtent (Collision|GetActorBounds (.ReturnValue (Actor|FindNearestActor InLocation (.FilteredSnapPoints (CallFunction|FilterSnapPoints _outactors "(GameplayTags=((TagName=\"Snap.Support\")))")))) false false)))))) InRotation InScale))
        (else
          (return false ""))))))

(fn ProcessNewTile
  (params (Tile%20Reference :type BP%20Build%20Master%20Object%20Reference) (TileType :type ETileName%20Enum :default "NewEnumerator1"))
  (switch Utilities|FlowControl|Switch|SwitchonETileName TileType
    (:NewEnumerator1
      (Utilities|NewCapsuleSnap (Transformation|GetActorLocation Tile%20Reference) (* (.z (.BoxExtent (Collision|GetActorBounds Tile%20Reference false false))) 2.0) (Variables|Constants|GetCellSideLength)))))

(fn FilterSnapPoints
  (params (Actors :type Array%20of%20Actor%20Object%20References) (Tags :type Gameplay%20Tag%20Container%20Structure))
  (bind _filteredsnaps (LocalVariables|GetFilteredSnaps))
  (for _array_element Actors
    (if (Utilities|DoesObjectImplementInterface _array_element "/Game/BuildingSystem/Blueprints/BPI_BuildInterface.BPI_BuildInterface_C")
      (bind _tags (Class|BPIBuildInterface|GetSnapPointTags(Message) _array_element))
      (if (GameplayTags|HasAnyTags _tags Tags true)
        (Utilities|Array|AddUnique (LocalVariables|GetFilteredSnaps) _array_element))))
  (return _filteredsnaps (> (Utilities|Array|Length _filteredsnaps) 0)))